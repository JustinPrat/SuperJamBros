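; Character Blueprint for Jammus that hooks up the character's special move state to a gun and a charged energy ball.
; The construction script assigns the SpaceGun to the special move state component as its gun.
; BeginPlay binds the state's start, exit and tick delegates.
; Start shows and exit hides the energy ball instance, each with a debug print, while tick is left empty.
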(event `self.ReceiveBeginPlay`
  (bind _smashcharacterstatespecialmove (`self.SmashCharacterStateSpecialMove`))
  (add `SmashCharacterStateSpecialMove.StartSpecialMoveDelegate` _smashcharacterstatespecialmove (delegate `StartSpecialMoveDelegate_Event`))
  (add `SmashCharacterStateSpecialMove.ExitSpecialMoveDelegate` _smashcharacterstatespecialmove (delegate `ExitSpecialMoveDelegate_Event`))
  (add `SmashCharacterStateSpecialMove.TickSpecialMoveDelegate` _smashcharacterstatespecialmove (delegate `TickSpecialMoveDelegate_Event`)))

(event `StartSpecialMoveDelegate_Event`
  (params (PreviousStateID :type "ESmashCharacterStateID Enum" :default "None"))
  (`self.SetActorHiddenInGame` (`SmashCharacterStateSpecialMove.EnergyBallInstance` (`self.SmashCharacterStateSpecialMove`)) false)
  (`KismetSystemLibrary.PrintString` "STARTCharge"))

(event `ExitSpecialMoveDelegate_Event`
  (params (NextStateID :type "ESmashCharacterStateID Enum" :default "None"))
  (`self.SetActorHiddenInGame` (`SmashCharacterStateSpecialMove.EnergyBallInstance` (`self.SmashCharacterStateSpecialMove`)) true)
  (`KismetSystemLibrary.PrintString` "STOPCharge"))

(event `TickSpecialMoveDelegate_Event`
  (params (DeltaTime :type "Float (single-precision)")))

(fn `UserConstructionScript`
  (set `SmashCharacterStateSpecialMove.Gun` (`self.SpaceGun`) (`self.SmashCharacterStateSpecialMove`)))